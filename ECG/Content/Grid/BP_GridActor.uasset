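; BP_GridActor builds a staggered grid of cells when play begins.
; Generate loops over X and Y, spaces cells by CellSize, shifts alternating ones by an offset and passes each to CreateNewCell.
; OnUpdateEntityPlace adds a static mesh component at the given cell's location plus a spawn offset.
; GenerateTest repeats the layout using mesh components directly, and PrintAllCellData calls GetCellData on each cell's entity.
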(event EventBeginPlay
  (CallFunction|Generate))

(event EventOnUpdateEntityPlace
  (params (InEntity :type Entity%20Wrapper%20Structure%20%28by%20ref%29) (GridCell :type Grid%20Cell%20Structure%20%28by%20ref%29))
  (AddComponent|AddStaticMeshComponent false (Math|Conversions|ToTransform(Vector) (+ (Variables|/Script/Engine.SceneComponent|GetRelativeLocation (.MeshComponent (Utilities|Struct|BreakGridCell GridCell))) (Variables|Default|GetEntitySpawnOffset)))))

(fn ConstructionScript)

(fn Generate
  (bind _cellsize (Variables|Default|GetCellSize))
  (bind (_x _y) (Math|Vector|BreakVector _cellsize))
  (for _index (range 0 (- (Variables|Default|GetY) 1))
    (for _index_2 (range 0 (- (Variables|Default|GetX) 1))
      (bind _output_get (LocalVariables|SetCellLocation (+ (select (== (Math|Integer|%(Integer) _index_2 2) 0) (Variables|Default|GetAdditianalOffset) "0, 0, 0") (Math|Vector|MakeVector (* _index _x) (* _y _index_2) 0.0))))
      (Class|GridActor|CreateNewCell _index_2 _index _output_get (Transformation|GetActorRotation) (Class|KismetMathLibrary|VectorOne)))))

(fn GenerateTest
  (bind _cellsize (Variables|Default|GetCellSize))
  (bind (_x _y) (Math|Vector|BreakVector _cellsize))
  (for _index (range 0 (- (Variables|Default|GetY) 1))
    (for _index_2 (range 0 (- (Variables|Default|GetX) 1))
      (bind _output_get (LocalVariables|SetCellLocation (+ (select (== (Math|Integer|%(Integer) _index_2 2) 0) (Variables|Default|GetAdditianalOffset) "0, 0, 0") (Math|Vector|MakeVector (* _index _x) (* _y _index_2) 0.0))))
      (AddComponent|AddBPCellMeshComponent false (Math|Transform|MakeTransform _output_get (Transformation|GetActorRotation))))))

(fn PrintAllCellData
  (for _array_element (Variables|Default|GetCells)
    (Class|GridActor|GetCellData (Variables|/Script/Common.CellMeshComponent|GetEntity _array_element))))